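; BP_BaseInteractiveObject is a base interactive object that shows or hides an outline on its static mesh.
; Each Tick it reads the ShouldOutline flag and calls AddObjectOutline or RemoveObjectOutline.
; Both toggle the mesh's Render Custom Depth, presumably for an outline post-process, and a HasOutlined flag keeps the add from repeating.
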(event EventBeginPlay)

(event EventTick
  (params (DeltaSeconds :type Float%20%28single-precision%29))
  (if (Variables|Default|GetbShouldOutline)
    (CallFunction|AddObjectOutline)
    (else
      (CallFunction|RemoveObjectOutline))))

(fn ConstructionScript)

(fn AddObjectOutline
  (if (not (Variables|Default|GetbHasOutlined))
    (Variables|Default|SetbHasOutlined true)
    (Rendering|SetRenderCustomDepth (Variables|Default|GetStaticMesh) true)))

(fn RemoveObjectOutline
  (Rendering|SetRenderCustomDepth (Variables|Default|GetStaticMesh) false)
  (Variables|Default|SetbHasOutlined false))