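; First-person player character for an espionage adventure, handling movement, interactable highlighting, physics grabbing and on-screen messages; Fire and Action are empty stubs.
; Each tick, a camera sphere trace outlines the hit BP_BaseInteractiveObject and displays its text.
; Grab uses CSGrabber's trace and a PhysicsHandle, gated by a Q-toggled grabber mode.
; DisplayMessage drives WBP_DisplayData with a restartable hide timer, optionally disabling input, as for the BeginPlay welcome.
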(event EventBeginPlay
  (bind _returnvalue (Game|GetPlayerController 0))
  ;[1 1 1] Begin Play ( Setup some stuff )
  (Utilities|FlowControl|Sequence
    (:then_0
      (Utilities|Array|Add (Variables|Default|GetIgnoredActors) self))
    (:then_1
      (bind _returnvalue_2 (UserInterface|CreateWidget "/Game/UI/WBP_Crosshair.WBP_Crosshair_C" _returnvalue))
      (UserInterface|Viewport|AddtoViewport _returnvalue_2 0))
    (:then_2
      (bind _returnvalue_3 (UserInterface|CreateWidget "/Game/UI/WBP_DisplayData.WBP_DisplayData_C" _returnvalue))
      (UserInterface|Viewport|AddtoViewport _returnvalue_3 0))
    (:then_3
      (CallFunction|DisplayMessage "Welcome Earthling.." "Hello, and welcome to a fun excited espionage adventure! [Experimental] Controller input is disabled while this message is displayed." "-AlienDude42" 3.0 true))))

(event EventTick
  (params (DeltaSeconds :type Float%20%28single-precision%29))
  ;[1 1 1] Check if player is looking at an interactable object every tick.
  (CallFunction|ChecktoSeeifPlayerIsLookingatObject))

(event Input|ActionEvents|InputActionCrouch
  (params (Key :type Key%20Structure))
  ;[1 1 1] Action Mappings
  (:Pressed
    (CallFunction|BeginCrouch))
  (:Released
    (CallFunction|EndCrouch)))

(event Input|ActionEvents|InputActionFire
  (params (Key :type Key%20Structure))
  ;[1 1 1] Action Mappings
  (:Pressed
    (CallFunction|Fire)))

(event Input|ActionEvents|InputActionGrab
  (params (Key :type Key%20Structure))
  (:Pressed
    (if (Variables|/Script/EspionageGame.CSGrabber|GetbGrabberModeEnabled (Variables|Default|GetCSGrabber))
      (CallFunction|RequestGrab)))
  (:Released
    (CallFunction|Release)))

(event Input|ActionEvents|InputActionJump
  (params (Key :type Key%20Structure))
  ;[1 1 1] Action Mappings
  (:Pressed
    (Character|Jump)))

(event Input|AxisEvents|InputAxisMoveForward
  (params (AxisValue :type Float%20%28single-precision%29))
  ;[1 1 1] Axis Mappings
  (CallFunction|MoveForward AxisValue))

(event Input|AxisEvents|InputAxisMoveRight
  (params (AxisValue :type Float%20%28single-precision%29))
  ;[1 1 1] Axis Mappings
  (CallFunction|MoveRight AxisValue))

(event Input|AxisEvents|InputAxisLookUp
  (params (AxisValue :type Float%20%28single-precision%29))
  ;[1 1 1] Axis Mappings
  (Pawn|Input|AddControllerPitchInput AxisValue))

(event Input|AxisEvents|InputAxisTurn
  (params (AxisValue :type Float%20%28single-precision%29))
  ;[1 1 1] Axis Mappings
  (Pawn|Input|AddControllerYawInput AxisValue))

(event Input|KeyboardEvents|Q
  (params (Key :type Key%20Structure))
  (bind _csgrabber (Variables|Default|GetCSGrabber))
  ;[1 1 1] Action Mappings
  (:Pressed
    (Variables|/Script/EspionageGame.CSGrabber|SetbGrabberModeEnabled _csgrabber (not (Variables|/Script/EspionageGame.CSGrabber|GetbGrabberModeEnabled _csgrabber)))
    (CallFunction|DisplayMessage "DEBUG DATA" (Utilities|String|Append "Grabber Mode: " (Utilities|String|ToString(Boolean) (Variables|/Script/EspionageGame.CSGrabber|GetbGrabberModeEnabled _csgrabber))) "-Internal System" 3.0 false)))

(fn ConstructionScript)

(fn MoveForward
  (params (Value :type Float%20%28single-precision%29))
  (Pawn|Input|AddMovementInput (Transformation|GetActorForwardVector) Value false))

(fn MoveRight
  (params (Value :type Float%20%28single-precision%29))
  (Pawn|Input|AddMovementInput (Transformation|GetActorRightVector) Value false))

(fn BeginCrouch
  (Character|Crouch))

(fn EndCrouch
  (Character|UnCrouch))

(fn Fire)

(fn Action)

(fn ChecktoSeeifPlayerIsLookingatObject
  ;[1 1 1] Cast a Sphere Trace from the Camera ignoring the player and see if we are looking at an interactable object.
  (bind (_outhit _returnvalue) (CallFunction|InteractiveHitScan (Variables|Default|GetObjectType) "None"))
  (if _returnvalue
    (CallFunction|NotifyObjectPlayerIsLookingatIt _outhit)
    (else
      (CallFunction|NotifyObjectPlayerIsNoLongerLookingatIt))))

(fn NotifyObjectPlayerIsLookingatIt
  (params (Hit :type Hit%20Result%20Structure))
  ;[1 1 1] Cast to the Object we hit, and tell it to outline. Also get the data stored on the object and display it on the screen.
  (Utilities|FlowControl|Sequence
    (:then_0
      (bind _asbp_base_interactive_object (Utilities|Casting|CastToBP_BaseInteractiveObject (.HitActor (Collision|BreakHitResult Hit))))
      (bind _output_get (Variables|Default|SetHitObject _asbp_base_interactive_object))
      (Variables|/Game/Blueprints/Objects/BP_BaseInteractiveObject.BP_BaseInteractiveObject_C|SetbShouldOutline _output_get true))
    (:then_1
      (CallFunction|DisplayMessage (Utilities|String|ToString(Text) (Variables|/Game/Blueprints/Objects/BP_BaseInteractiveObject.BP_BaseInteractiveObject_C|GetDisplay%20Title _asbp_base_interactive_object)) (Utilities|String|ToString(Text) (Variables|/Game/Blueprints/Objects/BP_BaseInteractiveObject.BP_BaseInteractiveObject_C|GetDisplay%20Message _asbp_base_interactive_object)) (Utilities|String|ToString(Text) (Variables|/Game/Blueprints/Objects/BP_BaseInteractiveObject.BP_BaseInteractiveObject_C|GetDisplayer%20Signature _asbp_base_interactive_object)) 3.0 false))))

(fn NotifyObjectPlayerIsNoLongerLookingatIt
  (bind _hitobject (Variables|Default|GetHitObject))
  ;[1 1 1] Remove outline on the object we are no longer looking at.
  (if (Utilities|IsValid _hitobject)
    (Variables|/Game/Blueprints/Objects/BP_BaseInteractiveObject.BP_BaseInteractiveObject_C|SetbShouldOutline _hitobject false)))

(fn DisplayMessage
  (params (DisplayTitle :type String) (DisplayMessage :type String) (DisplaySignature :type String) (DisplayDuration :type Float%20%28single-precision%29) (DisableControl :type Boolean))
  ;[1 1 1] Get data for message and display in UI
  (Utilities|Time|ClearandInvalidateTimerbyHandle (Variables|Default|GetTimerHandle_FlushDisplayMessage))
  (bind _foundwidgets (Widget|GetAllWidgetsOfClass "/Game/UI/WBP_DisplayData.WBP_DisplayData_C" true))
  (Default|UpdateDisplayData (Utilities|Array|Get(acopy) _foundwidgets) DisplayTitle DisplayMessage DisplaySignature)
  (bind _returnvalue (Utilities|Time|SetTimerbyFunctionName 0 "FlushDisplayMessage" DisplayDuration))
  (Variables|Default|SetTimerHandle_FlushDisplayMessage _returnvalue)
  (Default|UpdateDisplayVisibility (Utilities|Array|Get(acopy) _foundwidgets) true)
  (if DisableControl
    (Input|DisableInput (Game|GetPlayerController 0))))

(fn FlushDisplayMessage
  ;[1 1 1] Update Display Data Visiblity & Re-enable controller input if needed.
  (bind _foundwidgets (Widget|GetAllWidgetsOfClass "/Game/UI/WBP_DisplayData.WBP_DisplayData_C" true))
  (Default|UpdateDisplayVisibility (Utilities|Array|Get(acopy) _foundwidgets) false)
  (Input|EnableInput (Game|GetPlayerController 0)))

(fn InteractiveHitScan
  (params (ObjectTypes :type Array%20of%20EObjectTypeQuery%20Enums :default "ObjectTypeQuery1") (DrawDebugType :type EDrawDebugTrace%20Enum :default "None"))
  (bind _camera (Variables|Default|GetCamera))
  (bind _returnvalue (Transformation|GetWorldLocation _camera))
  (bind (_outhit _returnvalue_2) (Collision|SphereTraceForObjects _returnvalue (+ _returnvalue (* (Math|Vector|GetForwardVector _camera) (Variables|Default|GetReachRange))) (Variables|Default|GetObjectCheckRadius) ObjectTypes false (Variables|Default|GetIgnoredActors) DrawDebugType true "(R=1.000000,G=0.000000,B=0.000000,A=1.000000)" "(R=0.000000,G=1.000000,B=0.000000,A=1.000000)" 2e+01))
  (return _outhit _returnvalue_2))

(fn RequestGrab
  (bind _returnvalue (Class|CSGrabber|TryGrab (Variables|Default|GetCSGrabber)))
  (if (not (Collision|IsOverlappingActor (Variables|Default|GetCapsule) (.HitActor (Collision|BreakHitResult _returnvalue)) :!class /Script/Engine.PrimitiveComponent))
    (Utilities|IsValid (.HitActor (Collision|BreakHitResult _returnvalue))
      (:Is%20Valid
        (Physics|Components|PhysicsHandle|GrabComponentatLocationwithRotation (Variables|Default|GetPhysicsHandle) (.HitComponent (Collision|BreakHitResult _returnvalue)) "None" (Transformation|GetActorLocation (.HitActor (Collision|BreakHitResult _returnvalue))) (Transformation|GetActorRotation (.HitActor (Collision|BreakHitResult _returnvalue))))))))

(fn Release
  (Physics|Components|PhysicsHandle|ReleaseComponent (Variables|Default|GetPhysicsHandle)))